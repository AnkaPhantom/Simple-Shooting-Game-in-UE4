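; BP_TrackerBot is a tracker bot Blueprint holding test logic for pursuing the player, none of which is currently wired to run.
; FindNextPathPoint computes a navigation path to the player pawn and draws debug spheres at its points.
; Disconnected nodes would call that event, scale audio volume by the bot's speed with a printed readout, or move it toward the player via SimpleMoveToActor.
; Tick and the construction script are empty.
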(event `Find Next Path Point`
  ;[1 1 1] Blueprints of Find Next Path Point
  (bind _returnvalue (`NavigationSystemV1.FindPathToActorSynchronously` (`self.K2_GetActorLocation`) (`GameplayStatics.GetPlayerPawn` 0) 50.0 null null))
  (for _array_element (`NavigationPath.PathPoints` _returnvalue)
    (`KismetSystemLibrary.DrawDebugSphere` _array_element 20.0 12 (struct :`R` 1.0 :`G` 0.700368 :`B` 0.168039 :`A` 1.0) 6.0 1.0)))

(event `self.ReceiveTick`
  (params (DeltaSeconds :type "Float (single-precision)")))

(fn `UserConstructionScript`)